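; Collectable crystal actor that gets pulled into the player when they overlap it, then destroys itself.
; On overlap, an IsPlayer macro filters for the player pawn, then the starting location, scale and light intensity are stored.
; A timeline drives lerps that home the crystal on the pawn's current location, shrink it to zero and fade its light on a separate curve.
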(event Collision|EventActorBeginOverlap
  (params (OtherActor :type Actor%20Object%20Reference))
  (Utilities|IsPlayer OtherActor
    (:Is%20Player
      (CallFunction|StoreStartingValues)
      (bind (_direction _smooth_lerp_alpha _light_intensity) (Timeline|TL_BlendAlpha Play)
        (:Update
          (CallFunction|MovetoPlayer _smooth_lerp_alpha)
          (CallFunction|ScaleCrystal _smooth_lerp_alpha)
          (CallFunction|ChangeLightIntencity _light_intensity))
        (:Finished
          (Actor|DestroyActor))))))

(fn ConstructionScript)

(fn MovetoPlayer
  (params (Alpha :type Float%20%28single-precision%29))
  (Transformation|SetActorLocation (Math|Vector|Lerp(Vector) (Variables|Default|GetLerpStartLocation) (Transformation|GetActorLocation (Game|Player|GetPlayerPawn 0)) Alpha) false false))

(fn StoreStartingValues
  (Variables|Default|SetLerpStartLocation (Transformation|GetActorLocation))
  (Variables|Default|SetStartScale (Transformation|GetActorScale3D))
  (Variables|Default|SetStart%20Light%20Intencity (Variables|/Script/Engine.LightComponentBase|GetIntensity (Variables|Default|GetCrystalLight))))

(fn ScaleCrystal
  (params (Alpha :type Float%20%28single-precision%29))
  (Transformation|SetActorScale3D (Math|Vector|Lerp(Vector) (Variables|Default|GetStartScale) "0, 0, 0" Alpha)))

(fn ChangeLightIntencity
  (params (Alpha :type Float%20%28single-precision%29))
  (Rendering|Components|Light|SetIntensity (Variables|Default|GetCrystalLight) (Math|Float|Lerp (Variables|Default|GetStart%20Light%20Intencity) 0.0 Alpha)))