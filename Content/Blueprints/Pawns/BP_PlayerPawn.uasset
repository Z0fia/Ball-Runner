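; Player pawn that moves by applying physics torque to its mesh and restarts the level when it takes any damage.
; Forward/backward and right/left axis inputs drive torque around the Y and X axes.
; The camera fades in on BeginPlay.
; Damage calls Restart Lvl, which uses DoOnce to fade the camera out a single time, then reopens the current level by name after the fade.
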(event EventBeginPlay
  (CameraFades|StartCameraFade :self (Game|GetPlayerCameraManager 0) :FromAlpha 1.0 :Duration 0.5))

(event Collision|EventActorBeginOverlap
  (params (OtherActor :type Actor%20Object%20Reference)))

(event EventTick
  (params (DeltaSeconds :type Float%20%28single-precision%29)))

(event Game|Damage|EventAnyDamage
  (params (Damage :type Float%20%28single-precision%29) (DamageType :type Damage%20Type%20Object%20Reference) (InstigatedBy :type Controller%20Object%20Reference) (DamageCauser :type Actor%20Object%20Reference))
  (Utilities|RestartLvl))

(event Input|AxisEvents|InputAxisMoveForeward/Backward
  (params (AxisValue :type Float%20%28single-precision%29))
  (Class|PrimitiveComponent|AddTorqueinRadians (Variables|Default|GetPlayerPawn_Mesh) (Math|Vector|MakeVector 0.0 (* AxisValue 3e+06) 0.0) "None" false))

(event Input|AxisEvents|InputAxisMoveRight/Left
  (params (AxisValue :type Float%20%28single-precision%29))
  (Class|PrimitiveComponent|AddTorqueinRadians (Variables|Default|GetPlayerPawn_Mesh) (Math|Vector|MakeVector (* AxisValue 3e+06) 0.0 0.0) "None" false))

(fn ConstructionScript)